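; Destructible crate block that cracks and then explodes as it takes projectile hits.
; Each TakeDamage call removes one health point; at zero it spawns a Niagara explosion at its location and destroys itself.
; Once health falls to the crack threshold, a DoOnce gate swaps in the cracked texture through UpdateTexture a single time.
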(event EventBeginPlay
  (|CallParentFunction) ; This node is disabled and will not be called.\nDrag off pins to build functionality.
)

(event Collision|EventActorBeginOverlap
  (params (OtherActor :type Actor%20Object%20Reference))
  (|CallParentFunction OtherActor) ; This node is disabled and will not be called.\nDrag off pins to build functionality.
)

(event EventTick
  (params (DeltaSeconds :type Float%20%28single-precision%29))
  (|CallParentFunction DeltaSeconds) ; This node is disabled and will not be called.\nDrag off pins to build functionality.
)

(event EventTakeDamage
  ;[1 1 1] Manages taking damages when hit by a projectile
  (bind _result (Math|Integer|DecrementInt (Variables|Default|GetHealthPoints)) ; Substract 1 HP each time a projectile hits the crate
    (:%20%20
      (if (<= _result 0) ; If we do not have HP left
        (Niagara|SpawnSystematLocation "/Game/TheMadScientist/Core/NS_Explosion.NS_Explosion" (Transformation|GetActorLocation))
        (Actor|DestroyActor)
        (elif (<= _result (Variables|Default|GetCrackThreshold))
          (Utilities|FlowControl|DoOnce false
            (:Completed
              (CallFunction|UpdateTexture "/Game/TheMadScientist/Art/Interactables/Crate/T_Crate_Cracked.T_Crate_Cracked"))))))))

(fn ConstructionScript
  (|CallParentFunction))